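; BP_PC_Main is the main player controller, setting up input and the HUD for the local player.
; On BeginPlay it adds the mouse look and default Enhanced Input contexts, switches to game-only input and creates W_MainHUD.
; It binds the third-person character's inventory slot-change event to highlight the matching slot in the HUD's inventory UI.
; Debug keys run console commands to set the frame rate cap and show performance stats.
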(event `self.ReceiveBeginPlay`
  (bind _returnvalue (pcsubsystem `EnhancedInputLocalPlayerSubsystem` self))
  (if (`self.IsLocalController`)
    (`EnhancedInputSubsystemInterface.AddMappingContext` _returnvalue "/Game/Input/IMC_MouseLook.IMC_MouseLook" 0 (struct))
    (`EnhancedInputSubsystemInterface.AddMappingContext` _returnvalue "/Game/Input/IMC_Default.IMC_Default" 0 (struct))
    (set `self.bShowMouseCursor` false)
    (`WidgetBlueprintLibrary.SetInputMode_GameOnly` self)
    (bind _returnvalue_2 (`|CreateWidget` "/Game/_Main/Blueprints/UI/W_MainHUD.W_MainHUD_C"))
    (bind _output_get (set `self.HUD` _returnvalue_2))
    (`UserWidget.AddToViewport` _output_get 0)
    (bind _asbp_third_person_character (cast `/Game/ThirdPerson/Blueprints/BP_ThirdPersonCharacter` (`self.K2_GetPawn`)))
    (add `InventoryComponent.OnSelectedSlotChanged` (`BaseCharacter.InventoryComponent` _asbp_third_person_character) (delegate `SetHighlight`))))

(event `Key|G`
  (params (Key :type "Key Structure"))
  (:`Pressed`
    (`KismetSystemLibrary.ExecuteConsoleCommand` "t.MaxFPS 240" null)))

(event `Key|F`
  (params (Key :type "Key Structure"))
  (:`Pressed`
    (`KismetSystemLibrary.ExecuteConsoleCommand` "stat fps" self)
    (`KismetSystemLibrary.ExecuteConsoleCommand` "stat unit" self)))

(event `SetHighlight`
  (params (SlotNumber :type Integer) (bIsSelected :type Boolean))
  (`/Game/_Main/Blueprints/UI/Inventory/W_InventoryUI.SetSlotSelected` (`/Game/_Main/Blueprints/UI/W_MainHUD.W_InventoryUI` (`self.HUD`)) SlotNumber bIsSelected))

(event `self.ReceiveEndPlay`
  (params (EndPlayReason :type "EEndPlayReason Enum" :default "Destroyed")))

(fn `UserConstructionScript`)