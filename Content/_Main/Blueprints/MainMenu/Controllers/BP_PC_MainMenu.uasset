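; Main menu player controller that either joins a pending online session or shows the main menu.
; On BeginPlay it reads SessionToJoin from BP_GameInstance and, if valid on the local controller, calls JoinSession and clears the stored session on success or failure.
; Otherwise, the local controller creates W_MainMenu and adds it to the viewport, so a failed join does not open the menu.
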(event `self.ReceiveBeginPlay`
  (bind _returnvalue (`self.IsLocalController`))
  (bind _asbp_game_instance (cast `/Game/_Main/Blueprints/BP_GameInstance` (`GameplayStatics.GetGameInstance`)))
  (set `self.GameInstance` _asbp_game_instance)
  (if (and (`AdvancedSessionsLibrary.IsValidSession` (`/Game/_Main/Blueprints/BP_GameInstance.SessionToJoin` (`self.GameInstance`))) _returnvalue)
    (`JoinSessionCallbackProxy.JoinSession` (`GameplayStatics.GetPlayerController` 0) (`/Game/_Main/Blueprints/BP_GameInstance.SessionToJoin` (`self.GameInstance`))
      (:`OnSuccess`
        _)
      (:`OnFailure`
        _))
    (set `/Game/_Main/Blueprints/BP_GameInstance.SessionToJoin` (struct) (`self.GameInstance`))
    (elif _returnvalue
      (bind _returnvalue_2 (`|CreateWidget` "/Game/_Main/Blueprints/MainMenu/UI/W_MainMenu.W_MainMenu_C"))
      (bind _output_get (set `self.MainMenu` _returnvalue_2))
      (`UserWidget.AddToViewport` _output_get 0))))

(fn `UserConstructionScript`)